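; BP_Small_Light is an interactable light item that the player can switch on and off.
; InteractObject flips a State flag and sets the PointLight intensity between zero and a fixed brightness.
; LookAt uses the item data component's ItemID to find its data table row, returning the item name as a message along with the static mesh.
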(event `/Game/Inventory/BPI_InteractObject.Interact Object`
  (params (NewParam :type "Pawn Object Reference"))
  (bind _pointlight (`self.PointLight`))
  (if (`self.State`)
    (`LightComponent.SetIntensity` _pointlight 0.0)
    (set `self.State` false)
    (else
      (`LightComponent.SetIntensity` _pointlight 5000.0)
      (set `self.State` true))))

(fn `Look At`
  (returns (Message :type Text) (`Static Mesh Component` :type "StaticMeshComponent Object Reference"))
  (bind (_itemid_datatable _itemid_rowname) (break `DataTableRowHandle` (`/Game/Inventory/BP_ItemDataComponent.ItemID` (`self.BP_ItemDataComponent`))))
  (bind _returnvalue (`|GetDataTableRow` _itemid_datatable _itemid_rowname)
    (:`then`
      (return (`.Name_8_FEB957354A1610EBB0852DBE5FFA520A` (break `/Game/Inventory/F_ItemStruct` _returnvalue)) (`self.StaticMesh`)))))

(fn `UserConstructionScript`)