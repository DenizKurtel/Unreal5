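; Cable item actor that stretches a spline mesh from its origin to the point under the player's cursor.
; A 0.01-second delay loop from BeginPlay updates the end, snapping to "Electric In" on custom-channel hits.
; Once StopCable clears Continue and the cable has length, the loop ends and attempts to attach an end static mesh.
; Helpers return the item's data-table name and the nearer electric socket location.
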(event `self.ReceiveBeginPlay`
  (bind _spline (`self.Spline`))
  (bind (_hitresult _returnvalue) (`PlayerController.GetHitResultUnderCursorByChannel` (`self.Controller`) "TraceTypeQuery1" true))
  (bind (_location _tangent) (`SplineComponent.GetLocationAndTangentAtSplinePoint` _spline 1 "Local"))
  (bind (_location_2 _tangent_2) (`SplineComponent.GetLocationAndTangentAtSplinePoint` _spline 0 "Local"))
  (bind (_hitresult_2 _returnvalue_2) (`PlayerController.GetHitResultUnderCursorByChannel` (`self.Controller`) "TraceTypeQuery4" true))
  (set `self.Controller` (`GameplayStatics.GetPlayerController` 0))
  (bind _returnvalue_3 (`AddComponent|NODE_AddSplineMeshComponent-0`))
  (bind _output_get (set `self.Mesh` _returnvalue_3))
  (`SplineMeshComponent.SetForwardAxis` _output_get "X" true)
  (`SceneComponent.K2_AttachToComponent` (`self.Mesh`) (`self.Spline`) "None" "KeepRelative" "KeepRelative" "KeepRelative" true)
  (`SplineComponent.SetLocationAtSplinePoint` (`self.Spline`) 0 (`self.K2_GetActorLocation`) "World" true)
  (if _returnvalue_2 :!label _label
    (set `self.Location` (`SceneComponent.GetSocketLocation` (`.HitComponent` (`GameplayStatics.BreakHitResult` _hitresult_2)) "Electric In"))
    (else
      (set `self.Location` (`.Location` (`GameplayStatics.BreakHitResult` _hitresult)))))
  (`SplineComponent.SetLocationAtSplinePoint` (`self.Spline`) 1 (`self.Location`) "World" true)
  (`SplineMeshComponent.SetStartAndEnd` (`self.Mesh`) _location_2 _tangent_2 _location _tangent true)
  (if (not (and (not (`self.Continue`)) (> (`SplineComponent.GetSplineLength` _spline) 0.5)))
    (`KismetSystemLibrary.Delay` 0.01)
    (goto _label)
    (elif _returnvalue
      (bind _returnvalue_4 (`AddComponent|NODE_AddStaticMeshComponent-2` :`RelativeTransform` (`KismetMathLibrary.MakeTransform` (`self.Location`))))
      (bind _returnvalue_5 (`SceneComponent.K2_AttachToComponent` _returnvalue_4 (`self.Mesh`) "None" "KeepRelative" "KeepRelative" "KeepRelative" true))
      (`KismetSystemLibrary.PrintString` (`KismetStringLibrary.Conv_BoolToString` _returnvalue_5)))))

(event `/Game/Inventory/BPI_InteractObject.Stop Cable`
  (params (Continue :type Boolean))
  (set `self.Continue` Continue))

(fn `Look At`
  (returns (Message :type Text) (`Static Mesh Component` :type "StaticMeshComponent Object Reference"))
  (bind (_itemid_datatable _itemid_rowname) (break `DataTableRowHandle` (`/Game/Inventory/BP_ItemDataComponent.ItemID` (`self.BP_ItemDataComponent`))))
  (bind _returnvalue (`|GetDataTableRow` _itemid_datatable _itemid_rowname)
    (:`then`
      (return (`.Name_8_FEB957354A1610EBB0852DBE5FFA520A` (break `/Game/Inventory/F_ItemStruct` _returnvalue)) (`self.Mesh`)))))

(fn `Prepare Cable`
  (params (`Static Mesh Component` :type "MeshComponent Object Reference"))
  (returns (Location :type "Vector Structure"))
  (bind _returnvalue_location (`KismetMathLibrary.BreakTransform` (`SceneComponent.GetSocketTransform` `Static Mesh Component` "Electric In" "RTS_World")))
  (bind _returnvalue_location_2 (`KismetMathLibrary.BreakTransform` (`SceneComponent.GetSocketTransform` `Static Mesh Component` "Electric Out" "RTS_World")))
  (bind _returnvalue (`self.K2_GetActorLocation`))
  (if (or (`SceneComponent.DoesSocketExist` `Static Mesh Component` "Electric Out") (`SceneComponent.DoesSocketExist` `Static Mesh Component` "Electric In"))
    (if (< (`KismetMathLibrary.Vector_Distance` _returnvalue_location_2 _returnvalue) (`KismetMathLibrary.Vector_Distance` _returnvalue_location _returnvalue))
      (return _returnvalue_location_2)
      (else
        (return _returnvalue_location)))
    (else
      (return (0.0 0.0 0.0)))))

(fn `UserConstructionScript`)