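; BPC_Status is a component that tracks health and handles damage and death for the actor that owns it.
; It caches its owner on BeginPlay, and InduceDamage subtracts from Health when CanBeDamaged is set, ignoring the damage type.
; At zero health or below, a BP_Player_Character owner only prints a death message if CanDie is set, while any other owner is destroyed.
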(event `self.ReceiveBeginPlay`
  (set `self.Owner` (`self.GetOwner`)))

(event `self.ReceiveTick`
  (params (DeltaSeconds :type "Float (single-precision)")))

(fn `InduceDamage`
  (params (Damage :type "Float (double-precision)") (`Damage Type` :type String))
  (bind _owner (`self.Owner`))
  (if (`self.Can Be Damaged`)
    (bind _output_get (set `self.Health` (- (`self.Health`) Damage)))
    (if (<= _output_get 0.0)
      (cast `/Game/Characters/Player_Character/BP_Player_Character` _owner
        (:`then`
          (if (`self.Can Die`)
            (`KismetSystemLibrary.PrintString` "Dead")))
        (:`CastFailed`
          (`Actor.K2_DestroyActor` _owner))))))