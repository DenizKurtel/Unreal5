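; BPC_Hud is an actor component that creates and controls the player's on-screen HUD widget.
; On BeginPlay it creates W_HUD, hands it the owner's status, interaction and inventory components, and adds it to the viewport.
; Its events and functions forward requests to the widget for inventory containers, the menu and interaction prompts.
; It also shows a "Build" mode message based on the player controller's build-mode flag.
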(event `self.ReceiveBeginPlay`
  (bind _returnvalue (`self.GetOwner`))
  (bind _returnvalue_2 (`|CreateWidget` "/Game/Widgets/W_HUD.W_HUD_C" (`GameplayStatics.GetPlayerController` 0) (`Actor.GetComponentByClass` _returnvalue "/Game/Blueprints/BPC_Status.BPC_Status_C") (`Actor.GetComponentByClass` _returnvalue "/Game/Blueprints/BPC_Interaction.BPC_Interaction_C") (`Actor.GetComponentByClass` _returnvalue "/Game/Blueprints/BPC_Inventory.BPC_Inventory_C")))
  (bind _output_get (set `self.HUD` _returnvalue_2))
  (`UserWidget.AddToViewport` _output_get 0))

(event `Show Inventory`
  (params (Inventory :type "/Game/Blueprints/BPC_Inventory Object Reference"))
  (`/Game/Widgets/W_HUD.Show Container` (`self.HUD`) Inventory))

(event `Show Menu`
  (`/Game/Widgets/W_HUD.Display Menu Event` (`self.HUD`)))

(fn `DisplayInteractWith`
  (params (Message :type Text))
  (bind _hud (`self.HUD`))
  (set `/Game/Widgets/W_HUD.Interact Name` Message _hud)
  (`/Game/Widgets/W_HUD.Interact Message Show` _hud))

(fn `DisplayMode`
  (bind _hud (`self.HUD`))
  (bind _asbp_player_controller (cast `/Game/Blueprints/BP_Player_Controller` (`GameplayStatics.GetPlayerController` 0)))
  (if (`/Game/Blueprints/BP_Player_Controller.Is Build Mode` _asbp_player_controller)
    (set `/Game/Widgets/W_HUD.Mode` "Build" _hud)
    (`/Game/Widgets/W_HUD. Mode Message Show` _hud)
    (else
      (set `/Game/Widgets/W_HUD.Mode` "" _hud)
      (`/Game/Widgets/W_HUD.Mode Message Hide` _hud))))

(fn `HideInteractWith`
  (`/Game/Widgets/W_HUD.Interact Message Hide` (`self.HUD`)))

(fn `HideMode`
  (`/Game/Widgets/W_HUD.Mode Message Hide` (`self.HUD`)))