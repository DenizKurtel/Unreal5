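; Building system component for BP_Default_Character, an unfinished draft of placing meshes in a build mode.
; BeginPlay caches the controller and owning character, and start/stop events toggle the build-mode flag.
; PreviewLoop moves a preview mesh to the cursor's visibility trace hit, but nothing live calls it.
; Item creation and deletion are empty, with mesh setup and spawn logic left disconnected; keys 1 and 2 only set test flags.
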(event `self.ReceiveBeginPlay`
  (set `self.Controller` (`GameplayStatics.GetPlayerController` 0))
  (bind _asbp_default_character (cast `/Game/Characters/Default_Character/BP_Default_Character` (`self.GetOwner`)))
  (set `self.Character` _asbp_default_character))

(event `self.ReceiveTick`
  (params (DeltaSeconds :type "Float (single-precision)")))

(event `Preview Loop`
  (bind (_hitresult _returnvalue) (`PlayerController.GetHitResultUnderCursorByChannel` (`self.Controller`) "TraceTypeQuery1" true))
  (if _returnvalue
    (set `self.Location` (0.0 0.0 0.0))
    (`|ExecutionSequence`
      (:`then_0`
        (`/Engine/EditorBlueprintResources/StandardMacros.DoOnce` false :!label _label))
      (:`then_1`
        (bind _output_get (set `self.Preview Transform` (`KismetMathLibrary.MakeTransform` (`.Location` (`GameplayStatics.BreakHitResult` _hitresult)))))
        (`SceneComponent.K2_SetWorldTransform` (`self.Preview Mesh`) _output_get false false)))))

(event `Reset`
  (goto _label :!via `Reset`))

(event `Start Preview`
  (params (`Look At Actor` :type "Actor Object Reference") (`Static Mesh Component` :type "MeshComponent Object Reference"))
  (set `self.Look at Actor` `Look At Actor`)
  (set `self.Static Mesh Component` `Static Mesh Component`))

(event `Key|One`
  (params (Key :type "Key Structure"))
  (:`Pressed`
    (set `self.test 1` true))
  (:`Released`
    (set `self.test 2` false)))

(event `Key|Two`
  (params (Key :type "Key Structure"))
  (:`Pressed`
    (set `self.test 2` true))
  (:`Released`
    (set `self.test 1` false)))

(event `Create Item`)

(event `Delete Item`)

(event `Start Build Mode`
  (set `self.Is Build Mode` true))

(event `Stop Build Mode`
  (set `self.Is Build Mode` false))