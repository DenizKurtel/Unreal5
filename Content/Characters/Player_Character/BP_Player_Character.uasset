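; BP_Player_Character is the player character Blueprint that sets up input and its gameplay components when play begins.
; On BeginPlay it adds the IMC_Mapping Enhanced Input context, has BP_Player_Controller run its setup, then passes that controller to the BPCBuild component to initialize building.
; The 1 key applies fixed damage through the BPCStatus component, apparently as a debug hook.
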(event `self.ReceiveBeginPlay`
  ;[1 1 1] Init
  (bind _asplayer_controller (cast `PlayerController` (`self.GetController`)))
  (bind _returnvalue (pcsubsystem `EnhancedInputLocalPlayerSubsystem` _asplayer_controller))
  (`/Engine/EditorBlueprintResources/StandardMacros.IsValid` _returnvalue
    (:`Is Valid`
      (`EnhancedInputSubsystemInterface.AddMappingContext` _returnvalue "/Game/Characters/Inputs/IMC_Mapping.IMC_Mapping" 0 (struct))
      (bind _asbp_player_controller (cast `/Game/Blueprints/BP_Player_Controller` (`self.GetController`)))
      (`/Game/Blueprints/BP_Player_Controller.Set Up Controller` _asbp_player_controller)
      (`/Game/Blueprints/BPC_Build.Set Up Build` (`self.BPC_Build`) _asbp_player_controller))))

(event `Key|One`
  (params (Key :type "Key Structure"))
  (:`Pressed`
    (`/Game/Blueprints/BPC_Status.InduceDamage` (`self.BPC_Status`) 10.0 "")))

(fn `UserConstructionScript`)