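; Inventory system Blueprint that so far holds only look-at interaction logic; add, remove and LookAt functions are empty.
; InteractionTrace sphere-traces from camera or character, chosen by FPC, storing the hit actor and showing its HUD message.
; The message hides when the same actor is hit again, not on a miss.
; Tick and Interact are empty, leaving trace and item-data InteractMessage calls unwired.
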(event `self.ReceiveTick`
  (params (DeltaSeconds :type "Float (single-precision)")))

(event `EnhancedInput|/Game/Characters/Inputs/Input_Action/IA_Interact`
  (params (ActionValue :type Boolean) (ElapsedSeconds :type "Float (double-precision)") (TriggeredSeconds :type "Float (double-precision)") (InputAction :type "InputAction Object Reference" :default "/Game/Characters/Inputs/Input_Action/IA_Interact.IA_Interact")))

(event `Interact`
  (params (Target :type "Actor Object Reference")))

(fn `AddToInventory`)

(fn `Interaction Trace`
  (bind _returnvalue (`GameplayStatics.GetPlayerCameraManager` 0))
  (bind _returnvalue_2 (`GameplayStatics.GetPlayerCharacter` 0))
  (bind _returnvalue_3 (`Actor.K2_GetActorLocation` _returnvalue_2))
  (bind _returnvalue_4 (`Actor.K2_GetActorLocation` _returnvalue))
  (if (`self.FPC`)
    ;[1 1 1] FPC
    (set `self.Start` _returnvalue_4)
    (set `self.End` (+ _returnvalue_4 (* (`Actor.GetActorForwardVector` _returnvalue) (`self.InteractionRange`))))
    (else
      ;[1 1 1] TPC
      (set `self.Start` _returnvalue_3)
      (set `self.End` (+ _returnvalue_3 (* (`Actor.GetActorForwardVector` _returnvalue_2) (`self.InteractionRange`))))))
  (bind (_outhit _returnvalue_5) (`KismetSystemLibrary.SphereTraceSingle` (`self.Start`) (`self.End`) 15.0 "TraceTypeQuery3" false (`|MakeArray` (`self.GetOwner`))))
  (if _returnvalue_5
    (bind (_bblockinghit _binitialoverlap _time _distance _location _impactpoint _normal _impactnormal _physmat _hitactor) (`GameplayStatics.BreakHitResult` _outhit))
    (if (!= (`self.Look at Actor`) _hitactor)
      (bind _output_get (set `self.Look at Actor` _hitactor))
      (bind _message (message `/Game/Inventory/BPI_InteractInterface.Look At` _output_get))
      (message `/Game/Characters/Default_Character/BPI_Default_Character.Character Show HUD Interact` (`GameplayStatics.GetPlayerCharacter` 0) _message)
      (else
        (message `/Game/Characters/Default_Character/BPI_Default_Character.Character Hide HUD Interact` (`GameplayStatics.GetPlayerCharacter` 0))))
    (else
      (set `self.Look at Actor` null))))

(fn `Look At`)

(fn `RemoveFromInventory`)