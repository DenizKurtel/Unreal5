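; BP_Small_Light is a small light item that toggles on and off when interacted with.
; InteractObject flips a State flag and switches the PointLight intensity between zero and a fixed brightness.
; LookAt uses the item data component's row handle to return the item's data table name and its static mesh.
; PrepareCable is a stub that returns a zero vector.
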(event `/Game/Inventory/BPI_InteractObject.Interact Object`
  (bind _pointlight (`self.PointLight`))
  (if (`self.State`)
    (`LightComponent.SetIntensity` _pointlight 0.0)
    (set `self.State` false)
    (else
      (`LightComponent.SetIntensity` _pointlight 5000.0)
      (set `self.State` true))))

(fn `Look At`
  (returns (Message :type Text) (`Static Mesh Component` :type "StaticMeshComponent Object Reference"))
  (bind (_itemid_datatable _itemid_rowname) (break `DataTableRowHandle` (`/Game/Inventory/BP_ItemDataComponent.ItemID` (`self.BP_ItemDataComponent`))))
  (bind _returnvalue (`|GetDataTableRow` _itemid_datatable _itemid_rowname)
    (:`then`
      (return (`.Name_8_FEB957354A1610EBB0852DBE5FFA520A` (break `/Game/Inventory/F_ItemStruct` _returnvalue)) (`self.StaticMesh`)))))

(fn `Prepare Cable`
  (params (`Static Mesh Component` :type "MeshComponent Object Reference"))
  (returns (Location :type "Vector Structure"))
  (return (0.0 0.0 0.0)))

(fn `UserConstructionScript`)