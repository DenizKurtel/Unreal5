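; Interactable door that either swings freely under physics or opens and closes on interaction when unlocked.
; Free doors enable physics simulation at BeginPlay and ignore interaction.
; Otherwise, a dot product against the player's position picks a swing direction away from them, and a FlipFlop plays or reverses a timeline that drives the yaw.
; LookAt returns the door's name from the item data component's data table row.
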(event `self.ReceiveBeginPlay`
  ;[1 1 1] Initiate Door
  (if (`self.IsFree`)
    (`PrimitiveComponent.SetSimulatePhysics` (`self.Door`) true)))

(event `/Game/Inventory/BPI_InteractObject.Interact Object`
  ;[1 1 1] Door Interaction
  (if (`self.IsFree`)
    _
    (elif (not (`self.Locked`))
      (if (not (`self.IsOpen`))
        (set `self.Direction` (`KismetMathLibrary.SelectFloat` -90.0 90.0 (> 0.0 (`KismetMathLibrary.Dot_VectorVector` (`KismetMathLibrary.GetDirectionUnitVector` (`self.K2_GetActorLocation`) (`self.K2_GetActorLocation` (`GameplayStatics.GetPlayerCharacter` 0))) (`self.GetActorForwardVector`))))))
      ;;[1 1 1] Animater Door
      (`/Engine/EditorBlueprintResources/StandardMacros.FlipFlop`
        (:`A`
          (bind (_direction _door_rotation) (`Timeline|Open Door` :!label _label)
            (:`Update`
              (`SceneComponent.K2_SetRelativeRotation` (`self.Door`) (`KismetMathLibrary.MakeRotator` 0.0 0.0 (`KismetMathLibrary.Lerp` 0.0 (`self.Direction`) _door_rotation)) false false))
            (:`Finished`
              (set `self.IsOpen` (not (`self.IsOpen`))))))
        (:`B`
          (goto _label :!via `Reverse`))))))

(fn `Look At`
  (returns (Message :type Text))
  (bind (_itemid_datatable _itemid_rowname) (break `DataTableRowHandle` (`/Game/Inventory/BP_ItemDataComponent.ItemID` (`self.BP_ItemDataComponent`))))
  (bind _returnvalue (`|GetDataTableRow` _itemid_datatable _itemid_rowname)
    (:`then`
      (return (`.Name_8_FEB957354A1610EBB0852DBE5FFA520A` (break `/Game/Inventory/F_ItemStruct` _returnvalue))))))

(fn `UserConstructionScript`)