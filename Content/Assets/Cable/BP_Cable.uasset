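; BP_Cable is a cable actor that draws a spline mesh from its own location toward the point under the player's cursor.
; BeginPlay creates the mesh on the spline, then moves the end point to the cursor hit and reshapes the mesh.
; A short Delay loop repeats this while Stop is true, then prints a debug string.
; IneteractCable sets Stop; InteractLocation stores a Location this graph never reads.
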(event `self.ReceiveBeginPlay`
  (bind _spline (`self.Spline`))
  (bind (_location _tangent) (`SplineComponent.GetLocationAndTangentAtSplinePoint` _spline 1 "Local"))
  (bind (_location_2 _tangent_2) (`SplineComponent.GetLocationAndTangentAtSplinePoint` _spline 0 "Local"))
  (set `self.Controller` (`GameplayStatics.GetPlayerController` 0))
  (bind _returnvalue (`AddComponent|NODE_AddSplineMeshComponent-0`))
  (bind _output_get (set `self.Mesh` _returnvalue))
  (`SplineMeshComponent.SetForwardAxis` _output_get "X" true)
  (`SceneComponent.K2_AttachToComponent` (`self.Mesh`) (`self.Spline`) "None" "KeepRelative" "KeepRelative" "KeepRelative" true)
  (`SplineComponent.SetLocationAtSplinePoint` (`self.Spline`) 0 (`self.K2_GetActorLocation`) "World" true)
  (`SplineComponent.SetLocationAtSplinePoint` (`self.Spline`) 1 (`.Location` (`GameplayStatics.BreakHitResult` (`PlayerController.GetHitResultUnderCursorByChannel` (`self.Controller`) "TraceTypeQuery1" true))) "World" true :!label _label)
  (`SplineMeshComponent.SetStartAndEnd` (`self.Mesh`) _location_2 _tangent_2 _location _tangent true)
  (if (`self.Stop`)
    (`KismetSystemLibrary.Delay` 0.01)
    (goto _label)
    (else
      (`KismetSystemLibrary.PrintString` "Hello"))))

(event `/Game/Inventory/BPI_InteractObject.Ineteract Cable`
  (params (Stop :type Boolean))
  (set `self.Stop` Stop))

(event `/Game/Inventory/BPI_InteractObject.Interact Location`
  (params (Location :type "Vector Structure"))
  (set `self.Location` Location))

(fn `UserConstructionScript`)